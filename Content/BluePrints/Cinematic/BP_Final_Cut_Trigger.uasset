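; BP_Final_Cut_Trigger is a box trigger that starts the game's final cutscene and then the post-game credits.
; It creates a level sequence player for the final cut on BeginPlay.
; When the player character overlaps the box, it disables input, destroys the character and plays the sequence.
; A timer set to the sequence's duration then adds the credits widget to the viewport and starts its scroll.
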(event OnComponentBeginOverlap(BoxCollision)
  (params (OverlappedComponent :type Primitive%20Component%20Object%20Reference) (OtherActor :type Actor%20Object%20Reference) (OtherComp :type Primitive%20Component%20Object%20Reference) (OtherBodyIndex :type Integer) (bFromSweep :type Boolean) (SweepResult :type Hit%20Result%20Structure%20%28by%20ref%29))
  (bind _returnvalue (Game|GetPlayerCharacter 0))
  (bind _cutscene (Variables|Default|GetCutscene))
  (if (== OtherActor _returnvalue)
    (Input|DisableInput _returnvalue (Game|GetPlayerController 0))
    (Actor|DestroyActor _returnvalue)
    (Sequencer|Player|Play _cutscene :!class /Script/MovieScene.MovieSceneSequencePlayer)
    (Utilities|Time|SetTimerbyEvent (delegate Custom|PostGameCredtit) (Class|TimeManagementBlueprintLibrary|ToSeconds(QualifiedFrameTime) (Media|MediaPlayer|GetDuration _cutscene)))))

(event Custom|PostGameCredtit
  (bind _returnvalue (UserInterface|CreateWidget "/Game/BluePrints/Cinematic/W_PostGame_Credits.W_PostGame_Credits_C" (Game|GetPlayerController 0)))
  (UserInterface|Viewport|AddtoViewport _returnvalue 0)
  (Default|BeginScroll _returnvalue 1.0))

(event EventBeginPlay
  (bind _returnvalue (Sequencer|Player|CreateLevelSequencePlayer "/Game/BluePrints/Cinematic/FInal_Cut_Sequence.FInal_Cut_Sequence"))
  (Variables|Default|SetCutscene _returnvalue))

(fn ConstructionScript)