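; BP_Altar is an interactable altar that plays a one-time cutscene once all three coloured gems have been found in the player's inventory.
; On interact, it scans the inventory by item display name, latches blue, red and green flags, and shows the matching gemstone components.
; With all three flags set, it disables input, hides the character's root component and plays Step1_sequence.
; A timer matching the sequence length restores input only.
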(event OnInteract(Interaction)
  (params (Character :type Main%20Character%20Object%20Reference))
  (bind _asbp_player_character (Utilities|Casting|CastToBP_PlayerCharacter Character))
  (for _array_element (Class|InventoryComponent|GetItems (Variables|/Game/BluePrints/Player/BP_PlayerCharacter.BP_PlayerCharacter_C|GetInventory _asbp_player_character))
    (CallFunction|CheckBlueStone _array_element)
    (Rendering|SetVisibility (Variables|Default|GetBlue_Gemstone) (Variables|Default|GetExist_BlueGem) false)
    (CallFunction|CheckRedStone _array_element)
    (Rendering|SetVisibility (Variables|Default|GetRed_Gemstone) (Variables|Default|GetExist_RedGem) false)
    (CallFunction|CheckGreenStone _array_element)
    (Rendering|SetVisibility (Variables|Default|GetGreen_GemStone) (Variables|Default|GetExist_GreenGem) false))
  (CallFunction|StartCinematic))

(event Custom|Check%20Green%20Stone
  (params (Item :type Item%20Object%20Reference))
  (if (Utilities|Enum|Equal(Enum) (Variables|/Script/GameJam_052021.Item|GetItemDisplayName Item) (Variables|Default|GetGreen_Gem))
    (Variables|Default|SetExist_GreenGem true)))

(event Custom|Check%20Blue%20Stone
  (params (Item :type Item%20Object%20Reference))
  (if (Utilities|Enum|Equal(Enum) (Variables|/Script/GameJam_052021.Item|GetItemDisplayName Item) (Variables|Default|GetBlue_Gem))
    (Variables|Default|SetExist_BlueGem true)))

(event Custom|CutSceneStart
  (bind _returnvalue (Game|GetPlayerCharacter 0))
  (bind _cazzin (Variables|Default|Getcazzin))
  ;[1 0.6239 0] Trigger CutScene
  (Input|DisableInput _returnvalue (Game|GetPlayerController 0))
  (Rendering|SetVisibility (Variables|/Script/Engine.Actor|GetRootComponent _returnvalue) false false)
  (Sequencer|Player|Play _cazzin :!class /Script/MovieScene.MovieSceneSequencePlayer)
  (Utilities|Time|SetTimerbyEvent (delegate Custom|Enable%20Movement) (Class|TimeManagementBlueprintLibrary|ToSeconds(QualifiedFrameTime) (Media|MediaPlayer|GetDuration _cazzin))))

(event Custom|Check%20Red%20Stone
  (params (Item :type Item%20Object%20Reference))
  (if (Utilities|Enum|Equal(Enum) (Variables|/Script/GameJam_052021.Item|GetItemDisplayName Item) (Variables|Default|GetRed_Gem))
    (Variables|Default|SetExist_RedGem true)))

(event Custom|Enable%20Movement
  ;[1 0.6239 0] Trigger CutScene
  (Input|EnableInput (Game|GetPlayerCharacter 0) (Game|GetPlayerController 0)))

(event Custom|start%20cinematic
  (if (Math|Boolean|ANDBoolean (Variables|Default|GetExist_BlueGem) (Variables|Default|GetExist_RedGem) (Variables|Default|GetExist_GreenGem) (not (Variables|Default|GetCutSceneDone?)))
    (Variables|Default|SetCutSceneDone? true)
    (CallFunction|CutSceneStart)))

(event EventBeginPlay
  (bind _returnvalue (Sequencer|Player|CreateLevelSequencePlayer "/Game/GeneralAssets/Cinematic/Step1_sequence.Step1_sequence"))
  (Variables|Default|Setcazzin _returnvalue))

(event Collision|EventActorBeginOverlap
  (params (OtherActor :type Actor%20Object%20Reference)))

(event EventTick
  (params (DeltaSeconds :type Float%20%28single-precision%29)))

(fn ConstructionScript)