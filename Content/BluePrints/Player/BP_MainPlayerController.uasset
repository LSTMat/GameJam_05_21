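; Player controller that opens the inventory and map screens in response to their input actions.
; Each press lazily creates its widget on first use, caches it for reuse and adds it to the viewport.
; It then shows the mouse cursor and switches to UI-only input focused on that widget, with no logic here for closing it.
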(event EventBeginPlay)

(event EventTick
  (params (DeltaSeconds :type Float%20%28single-precision%29)))

(event Input|ActionEvents|InputActionInventory
  (params (Key :type Key%20Structure :default "None"))
  (:Pressed
    (Utilities|IsValid (Variables|Default|GetInvenotry%20Widget)
      (:Is%20Valid
        _)
      (:Is%20Not%20Valid
        (bind _returnvalue (UserInterface|CreateWidget "/Game/UserInterface/WBP_Inventory.WBP_Inventory_C"))
        (Variables|Default|SetInvenotry%20Widget _returnvalue)))
    (UserInterface|Viewport|AddtoViewport (Variables|Default|GetInvenotry%20Widget) 0)
    (Variables|Default|SetbShowMouseCursor true)
    (Input|SetInputModeUIOnly self (Variables|Default|GetInvenotry%20Widget) "DoNotLock")))

(event Input|ActionEvents|InputActionMap
  (params (Key :type Key%20Structure :default "None"))
  (:Pressed
    (Utilities|IsValid (Variables|Default|GetMap%20Widget)
      (:Is%20Valid
        _)
      (:Is%20Not%20Valid
        (bind _returnvalue (UserInterface|CreateWidget "/Game/UserInterface/WBP_Map.WBP_Map_C"))
        (Variables|Default|SetMap%20Widget _returnvalue)))
    (UserInterface|Viewport|AddtoViewport (Variables|Default|GetMap%20Widget) 0)
    (Variables|Default|SetbShowMouseCursor true)
    (Input|SetInputModeUIOnly self (Variables|Default|GetMap%20Widget) "DoNotLock")))

(fn ConstructionScript)